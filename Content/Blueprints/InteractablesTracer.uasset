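; InteractablesTracer is a scene-based tracer that finds and highlights objects implementing InteractableInterface along its forward vector.
; Trace line-traces by object type with debug drawing, storing and highlighting a valid hit, but returns failure while an interactable is already held.
; Highlighting sets a "Highlighted" scalar on dynamic material instances in slot 0 of each primitive component.
; RemoveCurrentInteractable turns the highlight off, calls TryEndInteraction and clears the reference.
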(fn `RemoveCurrentInteractable`
  (`self.RemoveInteractableMaterial`)
  (`/Game/Blueprints/HelperFunctions.TryEndInteraction` (`self.CurrentInteractable`))
  (set `self.CurrentInteractable` null) ; Set to NULL.
)

(fn `RemoveInteractableMaterial`
  (bind _asactor (cast `Actor` (`KismetSystemLibrary.Conv_InterfaceToObject` (`self.CurrentInteractable`))))
  (for _array_element (`Actor.K2_GetComponentsByClass` _asactor "/Script/Engine.PrimitiveComponent")
    (bind _asmaterial_instance_dynamic (cast `MaterialInstanceDynamic` (`PrimitiveComponent.GetMaterial` _array_element 0)))
    (`MaterialInstanceDynamic.SetScalarParameterValue` _asmaterial_instance_dynamic "Highlighted" 0.0)))

(fn `SetInteractableMaterial`
  (params (Interactable :type "/Game/Blueprints/InteractableInterface Interface"))
  (bind _asactor (cast `Actor` (`KismetSystemLibrary.Conv_InterfaceToObject` Interactable)))
  (for _array_element (`Actor.K2_GetComponentsByClass` _asactor "/Script/Engine.PrimitiveComponent")
    (bind _returnvalue (`PrimitiveComponent.CreateDynamicMaterialInstance` _array_element 0 (`PrimitiveComponent.GetMaterial` _array_element 0)))
    (`MaterialInstanceDynamic.SetScalarParameterValue` _returnvalue "Highlighted" 1.0)
    (`PrimitiveComponent.SetMaterial` _array_element 0 _returnvalue)))

(fn `Trace`
  (returns (Success :type Boolean) (Interactable :type "/Game/Blueprints/InteractableInterface Interface") (HitResult :type "HitResult Structure"))
  (bind _returnvalue (`self.K2_GetComponentLocation`))
  (`/Engine/EditorBlueprintResources/StandardMacros.IsValid` (`KismetSystemLibrary.Conv_InterfaceToObject` (`self.CurrentInteractable`))
    (:`Is Valid`
      (return false null))
    (:`Is Not Valid`
      (bind (_outhit _returnvalue_2) (`KismetSystemLibrary.LineTraceSingleForObjects` :`Start` _returnvalue :`End` (+ _returnvalue (* (`self.GetForwardVector`) (`self.TraceDistance`))) :`ObjectTypes` (`self.ObjectTypes`) :`DrawDebugType` "ForOneFrame" :`TraceColor` (struct :`R` 0.021567 :`B` 1.0 :`A` 1.0) :`DrawTime` 0.3))
      (if _returnvalue_2
        (bind (_asinteractable_interface _bsuccess) (cast `/Game/Blueprints/InteractableInterface` (`.HitActor` (`GameplayStatics.BreakHitResult` _outhit)) :!pure true))
        (if _bsuccess
          (bind _output_get (set `self.CurrentInteractable` _asinteractable_interface))
          (`self.SetInteractableMaterial` _output_get))
        (return _bsuccess _output_get _outhit)
        (else
          (return false null _outhit))))))