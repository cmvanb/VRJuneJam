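; LineTracer is a scene-based tracer that finds Interactable objects in front of it.
; Its Trace function casts an object-type line trace from its world location along its forward vector for a set distance, with debug drawing briefly visible.
; On a hit, it casts the actor to Interactable, stores it as the current interactable, and returns success, the interactable and the hit result.
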(fn `Trace`
  (returns (Success :type Boolean) (Interactable :type "/Game/Blueprints/Interactable Interface") (HitResult :type "HitResult Structure"))
  (bind _returnvalue (`self.K2_GetComponentLocation`))
  (bind (_outhit _returnvalue_2) (`KismetSystemLibrary.LineTraceSingleForObjects` :`Start` _returnvalue :`End` (+ _returnvalue (* (`self.GetForwardVector`) (`self.TraceDistance`))) :`ObjectTypes` (`self.ObjectTypes`) :`DrawDebugType` "ForDuration" :`TraceColor` (struct :`R` 0.021567 :`B` 1.0 :`A` 1.0) :`DrawTime` 0.3))
  (if _returnvalue_2
    (bind (_asinteractable _bsuccess) (cast `/Game/Blueprints/Interactable` (`.HitActor` (`GameplayStatics.BreakHitResult` _outhit)) :!pure true))
    (bind _output_get (set `self.CurrentInteractable` _asinteractable))
    (return _bsuccess _output_get _outhit)
    (else
      (return false null _outhit))))