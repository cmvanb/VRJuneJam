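; HelperFunctions provides two helper functions for safely starting and ending interactions on interactable objects.
; TryBeginInteraction and TryEndInteraction check that the Interactable is valid before calling BeginInteraction, which receives the Interactor, or EndInteraction.
; TryEndInteraction returns whether the call was made, while TryBeginInteraction returns true even when the Interactable is invalid.
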(fn `TryBeginInteraction`
  (params (Interactable :type "/Game/Blueprints/InteractableInterface Interface") (Interactor :type "Object Object Reference"))
  (returns (Success :type Boolean))
  (`/Engine/EditorBlueprintResources/StandardMacros.IsValid` (`KismetSystemLibrary.Conv_InterfaceToObject` Interactable)
    (:`Is Valid`
      (`/Game/Blueprints/InteractableInterface.BeginInteraction` Interactable Interactor)
      (return true))
    (:`Is Not Valid`
      (return true))))

(fn `TryEndInteraction`
  (params (Interactable :type "/Game/Blueprints/InteractableInterface Interface"))
  (returns (Success :type Boolean))
  (`/Engine/EditorBlueprintResources/StandardMacros.IsValid` (`KismetSystemLibrary.Conv_InterfaceToObject` Interactable)
    (:`Is Valid`
      (`/Game/Blueprints/InteractableInterface.EndInteraction` Interactable)
      (return true))
    (:`Is Not Valid`
      (return false))))